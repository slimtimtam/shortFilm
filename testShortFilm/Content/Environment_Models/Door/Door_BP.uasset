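; Door Blueprint that animates a five-piece door opening, triggered on BeginPlay or through the OpenDoor event.
; Both triggers play the Open timeline from the start, whose vector tracks drive the relative locations of the mesh pieces without sweeping.
; The bottom piece follows its own track, while the top and lower side pairs each share a track, mirrored by negating X.
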(event `Open Door`
  (bind (_direction _bottom_piece _top _left_bottom) (`Timeline|Open` :!via `PlayFromStart` :!label _label)
    (:`Update`
      (`SceneComponent.K2_SetRelativeLocation` (`self.Door_polySurface11`) _bottom_piece false false)
      (`SceneComponent.K2_SetRelativeLocation` (`self.Door_polySurface14`) _top false false)
      (`SceneComponent.K2_SetRelativeLocation` (`self.Door_polySurface13`) (`KismetMathLibrary.MakeVector` (* (.x _top) -1.0) (.y _top) (.z _top)) false false)
      (`SceneComponent.K2_SetRelativeLocation` (`self.Door_polySurface15`) _left_bottom false false)
      (`SceneComponent.K2_SetRelativeLocation` (`self.Door_polySurface12`) (`KismetMathLibrary.MakeVector` (* (.x _left_bottom) -1.0) (.y _left_bottom) (.z _left_bottom)) false false))))

(event `self.ReceiveBeginPlay`
  (goto _label :!via `PlayFromStart`))

(fn `UserConstructionScript`)